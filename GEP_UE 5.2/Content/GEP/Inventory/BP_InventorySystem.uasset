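; Slot-based inventory component that stores item ID and quantity stacks for its owner.
; Adding fills stacks up to ItemData table limits, then uses empty slots, growing the array beyond InventorySize when full.
; SERVER_ events swap differing slots between inventories, clear whole slots, or spawn dropped items at a traced point before the owner.
; Transfers and removals broadcast updates through MC_Update; key 1 prints contents for debugging.
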(event `Key|One`
  (params (Key :type "Key Structure"))
  ;[1 1 1] 1= Show all items in inventory
  (:`Pressed`
    (`self.DEBUG_PRINTCONTENTS`)))

(event `self.ReceiveBeginPlay`
  (`self.CreateInventorySlots`))

(event `MC_Update`
  (`self.OnInventoryUpdate`))

(event `SERVER_TransferSlots`
  (params (SourceInventory :type "/Game/GEP/Inventory/BP_InventorySystem Object Reference") (SourceIndex :type Integer) (Destinationindex :type Integer))
  (`self.TransferSlots` SourceInventory SourceIndex Destinationindex))

(event `SERVER_Remove`
  (params (Index :type Integer) (RemoveWholeStack :type Boolean) (IsConsumed :type Boolean))
  (`self.RemoveFromInventory` Index RemoveWholeStack IsConsumed))

(event `SERVER_DropItem`
  (params (ItemID :type Name) (ItemQuantity :type Integer))
  (for _ (range ItemQuantity)
    (`|SpawnActorFromClass` (`.ItemClass_10_9BB6B40D4C95792F433F53B5624885A5` (break `/Game/GEP/Inventory/fItemStruct` (`self.GetItemData` ItemID))) (`KismetMathLibrary.MakeTransform` (`self.GetDropLocation`)) "Undefined" "MultiplyWithRoot" null null)))

(fn `AddToInventory`
  (params (ItemID :type Name) (ItemQuantity :type Integer))
  (returns (Success :type Boolean) (QuantityRemaining :type Integer))
  (locals (Local_QuantityRemaining :type Integer) (Local_HasFailed :type Boolean))
  (set `local.Local_QuantityRemaining` ItemQuantity)
  (while (and (> (`local.Local_QuantityRemaining`) 0) (not (`local.Local_HasFailed`)))
    (bind (_index _foundslot) (`self.FindSlot` (`local.ItemID`)))
    (if _foundslot
      (`self.AddToStack` _index 1)
      (`/Engine/EditorBlueprintResources/StandardMacros.DecrementInt` (`local.Local_QuantityRemaining`))
      (elif (`self.AnyEmptySlots`)
        (bind _success (`self.CreateNewStack` (`local.ItemID`) 1))
        (if _success
          (`/Engine/EditorBlueprintResources/StandardMacros.DecrementInt` (`local.Local_QuantityRemaining`))
          (else
            (set `local.Local_HasFailed` true)))
        (else
          (set `local.Local_HasFailed` true)))))
  (return (not (`local.Local_HasFailed`)) (`local.Local_QuantityRemaining`)))

(fn `AddToStack`
  (params (Index :type Integer) (Quantity :type Integer))
  (bind (_output_itemid _output_quantity) (break `/Game/GEP/Inventory/fSlotStruct` (`|GetArrayItem` (`self.Content`) Index)))
  (`KismetArrayLibrary.Array_Set` (`self.Content`) Index (make `/Game/GEP/Inventory/fSlotStruct` _output_itemid (+ _output_quantity (`local.Quantity`)))))

(fn `AnyEmptySlots`
  (returns (HasEmptySlot :type Boolean) (EmptyIndex :type Integer))
  ;[1 1 1] Check to see if the inventory has a spare empty slot.
  (for (_array_element _array_index) (`self.Content`)
    (if (== (`.Quantity_6_838BA7554CEF8B6E1745ABA4D8EB1B54` (break `/Game/GEP/Inventory/fSlotStruct` _array_element)) 0)
      (return true _array_index)))
  (bind _returnvalue (`KismetArrayLibrary.Array_Add` (`self.Content`)))
  (return true _returnvalue))

(fn `CreateInventorySlots`
  (while (> (`self.InventorySize`) (`KismetArrayLibrary.Array_Length` (`self.Content`)))
    (`KismetArrayLibrary.Array_Add` (`self.Content`))
    (`KismetSystemLibrary.PrintString` "Adding")))

(fn `CreateNewStack`
  (params (ItemID :type Name) (Quantity :type Integer))
  (returns (Success :type Boolean))
  (bind (_hasemptyslot _emptyindex) (`self.AnyEmptySlots`))
  (if _hasemptyslot
    (`KismetArrayLibrary.Array_Set` (`self.Content`) _emptyindex (make `/Game/GEP/Inventory/fSlotStruct` (`local.ItemID`) (`local.Quantity`)))
    (return true)
    (else
      (return false))))

(fn `DEBUG_PRINTCONTENTS`
  ;[1 1 1] For each item in inventory array, get the ID and quantity and print both out
  (for (_array_element _array_index) (`self.Content`)
    (bind (_itemid _quantity) (break `/Game/GEP/Inventory/fSlotStruct` _array_element))
    (`KismetSystemLibrary.PrintString` (`KismetStringLibrary.Concat_StrStr` (`KismetStringLibrary.Conv_IntToString` _array_index) ": " (`KismetStringLibrary.Conv_NameToString` _itemid) " = " (`KismetStringLibrary.Conv_IntToString` _quantity)))))

(fn `FindSlot`
  (params (ItemID :type Name))
  (returns (Index :type Integer) (FoundSlot :type Boolean))
  (bind _itemid (`local.ItemID`))
  (for (_array_element _array_index) (`self.Content`)
    (bind (_itemid_2 _quantity) (break `/Game/GEP/Inventory/fSlotStruct` _array_element))
    (if (== _itemid_2 _itemid)
      (if (> (`self.GetMaxStackSize` _itemid) _quantity)
        (return _array_index true))))
  (return -1 false))

(fn `GetDropLocation`
  (returns (Location :type "Vector Structure"))
  (bind _returnvalue (`self.GetOwner`))
  (bind _returnvalue_2 (+ (`Actor.K2_GetActorLocation` _returnvalue) (* (`KismetMathLibrary.RandomUnitVectorInConeInDegrees` (`Actor.GetActorForwardVector` _returnvalue)) 150.0)))
  (bind _outhit (`KismetSystemLibrary.LineTraceSingle` _returnvalue_2 (- _returnvalue_2 (0.0 0.0 500.0)) "TraceTypeQuery1"))
  (return (`.Location` (`GameplayStatics.BreakHitResult` _outhit))))

(fn `GetItemData`
  (params (ItemID :type Name))
  (returns (Data :type "/Game/GEP/Inventory/fItemStruct Structure"))
  (bind _returnvalue (`|GetDataTableRow` "/Game/GEP/Inventory/ItemData.ItemData" ItemID)
    (:`then`
      (return _returnvalue))))

(fn `GetMaxStackSize`
  (params (ItemID :type Name))
  (returns (StackSize :type Integer))
  (bind _returnvalue (`|GetDataTableRow` "/Game/GEP/Inventory/ItemData.ItemData" ItemID)
    (:`then`
      (return (`.StackSize_13_2B59A4294092D8EDD3BC4BBB7CD7A81A` (break `/Game/GEP/Inventory/fItemStruct` _returnvalue))))
    (:`RowNotFound`
      (return -1))))

(fn `RemoveFromInventory`
  (params (Index :type Integer) (RemoveWholeStack :type Boolean) (IsConsumed :type Boolean))
  (locals (Local_Item :type Name) (Local_Quantity :type Integer))
  (bind (_output_itemid _output_quantity) (break `/Game/GEP/Inventory/fSlotStruct` (`|GetArrayItem` (`self.Content`) Index)))
  (set `local.Local_Item` _output_itemid)
  (set `local.Local_Quantity` _output_quantity)
  (`|ExecutionSequence`
    (:`then_0`
      (`KismetArrayLibrary.Array_Set` (`self.Content`) (`local.Index`) (make `/Game/GEP/Inventory/fSlotStruct` "None"))
      (if (not (`local.IsConsumed`))
        (`self.SERVER_DropItem` (`local.Local_Item`) (`local.Local_Quantity`))))
    (:`then_1`
      (`self.MC_Update`))))

(fn `TransferSlots`
  (params (SourceInventory :type "/Game/GEP/Inventory/BP_InventorySystem Object Reference") (SourceIndex :type Integer) (Destinationindex :type Integer))
  (locals (LocalSlotContent :type "/Game/GEP/Inventory/fSlotStruct Structure"))
  (set `local.LocalSlotContent` (`|GetArrayItem` (`/Game/GEP/Inventory/BP_InventorySystem.Content` SourceInventory) SourceIndex))
  (if (< Destinationindex 0)
    _
    (elif (not (== (`.ItemID_2_0606B30248D01AF764230098A988C775` (break `/Game/GEP/Inventory/fSlotStruct` (`local.LocalSlotContent`))) (`.ItemID_2_0606B30248D01AF764230098A988C775` (break `/Game/GEP/Inventory/fSlotStruct` (`|GetArrayItem` (`self.Content`) (`local.Destinationindex`))))))
      (`KismetArrayLibrary.Array_Set` (`/Game/GEP/Inventory/BP_InventorySystem.Content` (`local.SourceInventory`)) (`local.SourceIndex`) (`|GetArrayItem` (`self.Content`) (`local.Destinationindex`)))
      (`KismetArrayLibrary.Array_Set` (`self.Content`) (`local.Destinationindex`) (`local.LocalSlotContent`))
      (`self.MC_Update`)
      (`self.MC_Update` (`local.SourceInventory`)))))